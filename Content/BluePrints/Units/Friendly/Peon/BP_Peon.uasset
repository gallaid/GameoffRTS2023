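; BP_Peon is a friendly worker unit that takes right-click orders to move or gather resources.
; Right-clicking a resource stores it and writes its type to the AI Blackboard; any other click writes a destination and resets the type to a default, also set on BeginPlay.
; GatherResource builds a one-entry transfer map from the resource's type name and gather rate, then a shared resource action takes it from the resource to the peon.
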(event `self.ReceiveBeginPlay`
  (`parent.ReceiveBeginPlay`)
  (`BlackboardComponent.SetValueAsEnum` (`AIBlueprintHelperLibrary.GetBlackboard` (`AIBlueprintHelperLibrary.GetAIController` self)) "TypeOfResoruceTarget" (enumliteral `/Game/BluePrints/Structs/Enums/Enum_Resources` "NewEnumerator5")))

(fn `Gather Resource`
  ;[1 1 1] Build Transfer Map, input Actors, function does the rest.
  (`/Game/BluePrints/FunctionLibs/ResourceFunctions.Resource Action: Take Map from Target` (`self.Current Resource`) self (`|MakeMap` (`/Game/BluePrints/Resources/BP_ResourceBase.TypeName` (`self.Current Resource`)) (`self.Rate for Gather`))))

(fn `RightClickedWhileSelected`
  (params (`Hit IN` :type "HitResult Structure"))
  (bind (_bblockinghit _binitialoverlap _time _distance _location _impactpoint _normal _impactnormal _physmat _hitactor) (`GameplayStatics.BreakHitResult` `Hit IN`))
  (bind _blackboard (`AIController.Blackboard` (`AIBlueprintHelperLibrary.GetAIController` self)))
  (bind _asbp_resource_base (cast `/Game/BluePrints/Resources/BP_ResourceBase` _hitactor)
    (:`then`
      (set `self.Current Resource` _asbp_resource_base)
      (bind _output_get (set `self.CurrentResouceEnum` (`/Game/BluePrints/Resources/BP_ResourceBase.Type` _asbp_resource_base)))
      (`BlackboardComponent.SetValueAsEnum` (`AIController.Blackboard` (`AIBlueprintHelperLibrary.GetAIController` self)) "TypeOfResoruceTarget" _output_get))
    (:`CastFailed`
      (`BlackboardComponent.SetValueAsVector` _blackboard "Destination" _location)
      (`BlackboardComponent.SetValueAsEnum` _blackboard "TypeOfResoruceTarget" (enumliteral `/Game/BluePrints/Structs/Enums/Enum_Resources` "NewEnumerator5")))))

(fn `UserConstructionScript`
  (`parent.UserConstructionScript`))