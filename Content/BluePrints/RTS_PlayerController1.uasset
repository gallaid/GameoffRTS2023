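; RTS player controller that adds the input mapping, shows the cursor and handles unit selection and move orders through the RTS_Camera pawn.
; Left-click press, hold and release go to BP_HUD, while Ctrl+click toggles the unit under the cursor in SelectedActors.
; Right click traces from the camera through the cursor and sends every selected unit to the hit.
; The controller's own single-click and box-trace drag selection paths are left unwired.
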(event `self.ReceiveBeginPlay`
  (bind _returnvalue (subsystem `EnhancedInputLocalPlayerSubsystem`))
  ;[0.05098 0.05098 0.05098] Add Mapping Context
  (`/Engine/EditorBlueprintResources/StandardMacros.IsValid` _returnvalue
    (:`Is Valid`
      (`EnhancedInputSubsystemInterface.AddMappingContext` _returnvalue "/Game/BluePrints/Input/IMC_Default.IMC_Default" 0 (struct))
      (set `self.bShowMouseCursor` true)
      (bind _asrts_camera (cast `/Game/BluePrints/RTS_Camera` (`GameplayStatics.GetPlayerPawn` 0)))
      (bind _output_get (set `self.RTSCamera Actor` _asrts_camera))
      (set `self.Main Camera` (`/Game/BluePrints/RTS_Camera.MainCamera` _output_get)))))

(event `EnhancedInput|/Game/BluePrints/Input/Actions/RightClick`
  (params (ActionValue :type Boolean) (ElapsedSeconds :type "Float (double-precision)") (TriggeredSeconds :type "Float (double-precision)") (InputAction :type "InputAction Object Reference" :default "/Game/BluePrints/Input/Actions/RightClick.RightClick"))
  (bind (_worldlocation _worlddirection) (`self.DeprojectMousePositionToWorld`))
  (:`Triggered`
    (if (> (`KismetArrayLibrary.Array_Length` (`self.Selected Actors`)) 0)
      (bind _outhit (`KismetSystemLibrary.LineTraceSingle` :`Start` (`SceneComponent.K2_GetComponentLocation` (`self.Main Camera`)) :`End` (+ _worldlocation (* _worlddirection 5000.0)) :`TraceChannel` "TraceTypeQuery2" :`bTraceComplex` true :`DrawDebugType` "Persistent"))
      (for _array_element (`self.Selected Actors`)
        (bind _asunit_base (cast `` _array_element))
        (`self.Move To` _asunit_base (`.Location` (`GameplayStatics.BreakHitResult` _outhit)))))))

(event `self.ReceiveTick`
  (params (DeltaSeconds :type "Float (single-precision)"))
  (if (`self.IsLeftMousePressed?`)
    (`/Game/BluePrints/BP_HUD.Left Mouse Held` (stale `EnhancedInput|/Game/BluePrints/Input/Actions/LeftClick` _asbp_hud))))

(event `EnhancedInput|/Game/BluePrints/Input/Actions/ControlLeftClick`
  (params (ActionValue :type Boolean) (ElapsedSeconds :type "Float (double-precision)") (TriggeredSeconds :type "Float (double-precision)") (InputAction :type "InputAction Object Reference" :default "/Game/BluePrints/Input/Actions/ControlLeftClick.ControlLeftClick"))
  (:`Triggered`
    (`self.Control Click`)))

(event `EnhancedInput|/Game/BluePrints/Input/Actions/LeftClick`
  (params (ActionValue :type Boolean) (ElapsedSeconds :type "Float (double-precision)") (TriggeredSeconds :type "Float (double-precision)") (InputAction :type "InputAction Object Reference" :default "/Game/BluePrints/Input/Actions/LeftClick.LeftClick"))
  (:`Started`
    (bind _asbp_hud (cast `/Game/BluePrints/BP_HUD` (`self.GetHUD`)))
    (set `self.IsLeftMousePressed?` true)
    (`/Game/BluePrints/BP_HUD.Get Left Button pressed` _asbp_hud))
  (:`Completed`
    (set `self.IsLeftMousePressed?` false)
    (`/Game/BluePrints/BP_HUD.Left Mouse Released` _asbp_hud)))

(fn `Check For Deselect`
  (params (`Actor Array` :type "Array of Actor Object Reference"))
  (for _array_element `Actor Array`
    (if (not (`KismetArrayLibrary.Array_Contains` (`self.Selected Actors`) _array_element))
      (`self.DeselectActor` _array_element))))

(fn `Control Click`
  (bind _hit (`self.Get Line Trace From Mouse`))
  (bind _asunit_base (cast `` (`.HitActor` (`GameplayStatics.BreakHitResult` _hit))))
  (if (`/Game/BluePrints/RTS_PlayerController1.IsSelected` _asunit_base)
    (`self.DeselectActor` (`.HitActor` (`GameplayStatics.BreakHitResult` _hit)))
    (else
      (`self.Select Actor` (`.HitActor` (`GameplayStatics.BreakHitResult` _hit))))))

(fn `DeselectActor`
  (params (`Deselect This Actor` :type "Actor Object Reference"))
  (bind _asunit_base (cast `` `Deselect This Actor`))
  (set `/Game/BluePrints/RTS_PlayerController1.IsSelected` false _asunit_base)
  (`KismetArrayLibrary.Array_RemoveItem` (`self.Selected Actors`) `Deselect This Actor`))

(fn `Draw Selection Box`
  (locals (StartDrag :type "Vector2D Structure")))

(fn `Left Click`
  (for _array_element (`self.Selected Actors`)
    (`self.DeselectActor` _array_element))
  (bind _hit (`self.Get Line Trace From Mouse`))
  (cast `` (`.HitActor` (`GameplayStatics.BreakHitResult` _hit)))
  (`self.Select Actor` (`.HitActor` (`GameplayStatics.BreakHitResult` _hit))))

(fn `Make Selection Vectors`
  (returns (`Box Vertex out` :type "Array of Vector Structure"))
  (locals (`2d Vectors` :type "Array of Vector2D Structure") (`Location Vectors` :type "Array of Vector Structure"))
  (bind (_mouse_position_ws_start_x _mouse_position_ws_start_y) (`KismetMathLibrary.BreakVector2D` (`self.Mouse Position WS Start`)))
  (bind (_mouse_position_ws_end_x _mouse_position_ws_end_y) (`KismetMathLibrary.BreakVector2D` (`self.Mouse Position WS End`)))
  (bind _returnvalue (`KismetMathLibrary.FMin` _mouse_position_ws_start_x _mouse_position_ws_end_x))
  (bind _returnvalue_2 (`KismetMathLibrary.FMin` _mouse_position_ws_start_y _mouse_position_ws_end_y))
  (bind _returnvalue_3 (`KismetMathLibrary.FMax` _mouse_position_ws_start_y _mouse_position_ws_end_y))
  (bind _returnvalue_4 (`KismetMathLibrary.FMax` _mouse_position_ws_start_x _mouse_position_ws_end_x))
  (bind _output_get (set `local.2d Vectors` (`|MakeArray` (`KismetMathLibrary.MakeVector2D` _returnvalue _returnvalue_2) (`KismetMathLibrary.MakeVector2D` _returnvalue _returnvalue_3) (`KismetMathLibrary.MakeVector2D` _returnvalue_4 _returnvalue_2) (`KismetMathLibrary.MakeVector2D` _returnvalue_4 _returnvalue_3))))
  (for _array_element _output_get
    (bind (_worldposition _worlddirection) (`GameplayStatics.DeprojectScreenToWorld` (`GameplayStatics.GetPlayerController` 0) _array_element))
    (bind _outhit (`KismetSystemLibrary.LineTraceSingle` :`Start` _worldposition :`End` (+ _worldposition (* _worlddirection 100000000.0)) :`TraceChannel` "TraceTypeQuery1" :`DrawDebugType` "ForDuration"))
    (`KismetArrayLibrary.Array_Add` (`local.Location Vectors`) (`.Location` (`GameplayStatics.BreakHitResult` _outhit))))
  (return (`local.Location Vectors`)))

(fn `Select Actor`
  (params (IncomingActor :type "Actor Object Reference"))
  (bind _asunit_base (cast `` IncomingActor))
  (set `/Game/BluePrints/RTS_PlayerController1.IsSelected` true _asunit_base)
  (`KismetArrayLibrary.Array_Add` (`self.Selected Actors`) IncomingActor)
  (`KismetSystemLibrary.PrintString` (`KismetStringLibrary.Concat_StrStr` "In Select Actor" (`KismetSystemLibrary.GetDisplayName` IncomingActor))))

(fn `Set Destination`
  (params (Destination :type "Vector Structure"))
  (for _array_element (`self.Selected Actors`)
    (bind _asbp_friendly_unit_base (cast `/Game/BluePrints/Map_Entities/Friendly/BP_Friendly_Unit_Base` _array_element))
    (`self.Move To` _asbp_friendly_unit_base (`local.Destination`))))

(fn `UserConstructionScript`)