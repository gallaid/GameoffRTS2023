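; BP_StoneResource is a child resource Blueprint representing a stone resource in the world.
; Its construction script runs the inherited ResourceSetUp with an enum value, then reads the "Stones" row of DT_Stones and assigns a random mesh from it to the static mesh component.
; On BeginPlay it calls the parent and sets TypeName to "Stone".
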(event `self.ReceiveBeginPlay`
  (`parent.ReceiveBeginPlay`)
  (set `self.TypeName` "Stone"))

(fn `UserConstructionScript`
  (`parent.UserConstructionScript`)
  (`self.Resource Set Up` "NewEnumerator2")
  (bind _returnvalue (`|GetDataTableRow` "/Game/BluePrints/DataTables/DT_Stones.DT_Stones" "Stones")
    (:`then`
      (`StaticMeshComponent.SetStaticMesh` (`self.StaticMesh`) (`KismetArrayLibrary.Array_Random` (`.StaticMesh_9_9BD35E994BEF66EF4A324088D7BBF128` (break `/Game/BluePrints/Structs/Resources/ST_ResourceVaration` _returnvalue)))))))