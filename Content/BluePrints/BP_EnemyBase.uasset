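; BP_EnemyBase is an enemy Blueprint, named as a base, that tracks the player and shows a health bar.
; Each Tick it calls PawnActions.LookAt on the player pawn and refreshes health bars through DamageUtilities.
; Tick also pins the health bar widget to a fixed world rotation.
; A looping projectile-firing chain remains in the graph but is unconnected, so this Blueprint never fires.
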(event `self.ReceiveBeginPlay`
  (`parent.ReceiveBeginPlay`))

(event `self.ReceiveTick`
  (params (DeltaSeconds :type "Float (single-precision)"))
  (`parent.ReceiveTick` DeltaSeconds)
  (`/Game/BluePrints/FunctionLibs/ActorComponents/PawnActions.LookAt` (`self.PawnActions`) self (`GameplayStatics.GetPlayerPawn` 0) (0.0 0.0 0.0))
  (`/Game/BluePrints/FunctionLibs/ActorComponents/DamageUtilities.update Non-Player-Health-Bars` (`self.DamageUtilities`) self)
  (`SceneComponent.K2_SetWorldRotation` (`self.Widget HealthBar`) (struct :`Pitch` 45.0 :`Yaw` -180.0) false false))

(fn `UserConstructionScript`)