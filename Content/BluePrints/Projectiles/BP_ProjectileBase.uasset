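; Base projectile Blueprint that delivers a stack of hits to combat actors it strikes.
; On collider hit, unless the player immunity check blocks it, it passes the stack, attacker and ammo type to the target's DamageUtilities and prints debug output.
; It destroys itself after those hits and after striking other valid actors.
; Speed and gravity setup is disconnected, as is the comparison inside the immunity function.
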(event `self.Collider.OnComponentHit`
  (params (HitComponent :type "PrimitiveComponent Object Reference") (OtherActor :type "Actor Object Reference") (OtherComp :type "PrimitiveComponent Object Reference") (NormalImpulse :type "Vector Structure") (Hit :type "HitResult Structure (by ref)"))
  ;[1 1 1] Checking various things to ignore damage
  (bind _output_get (set `self.Defender` OtherActor))
  (`/Engine/EditorBlueprintResources/StandardMacros.IsValid` _output_get
    (:`Is Valid`
      (if (not (and (`self.PlayerProjectile`) (== (`GameplayStatics.GetPlayerPawn` 0) OtherActor)))
        (bind _asbp_combat_actor_base (cast `/Game/BluePrints/Map_Entities/BP_CombatActorBase` OtherActor)
          (:`then`
            ;[1 0.1354 0.1374] Applies all the "hits" stacked on the projectile.
            (bind (_success _debug) (`/Game/BluePrints/FunctionLibs/ActorComponents/DamageUtilities.Apply Hit Stack` (`/Game/BluePrints/Map_Entities/BP_CombatActorBase.DamageUtilities` _asbp_combat_actor_base) (`self.Projectile Hit Stack`) (`self.Attacker`) _asbp_combat_actor_base (`self.Ammo Type Name`) false))
            (`KismetSystemLibrary.PrintString` _debug true true (struct :`G` 0.66 :`B` 1.0 :`A` 1.0) 10.0)
            (`self.K2_DestroyActor`))
          (:`CastFailed`
            (`self.K2_DestroyActor`)))))
    (:`Is Not Valid`
      (`KismetSystemLibrary.PrintString` "i'm dead"))))

(fn `UserConstructionScript`)