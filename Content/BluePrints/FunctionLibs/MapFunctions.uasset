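; Blueprint function library of helpers for editing maps with float values.
; The update functions cache a key's current value, remove the entry, then re-add it with the change applied.
; The capped variant runs the change through CapAndReturnExcess and returns the amount over the cap.
; The missing-key helpers add zero-valued entries, either for one key or for every key of another map.
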(fn `Add Key if Missing: Float`
  (params (Map :type "Map of Name to Float (double-precision)") (Key :type Name))
  (if (not (`.ReturnValue` (`BlueprintMapLibrary.Map_Find` Map Key)))
    (`BlueprintMapLibrary.Map_Add` (`local.Map`) (`local.Key`))))

(fn `Add Keys if They Are Missing: Float`
  (params (Map :type "Map of Name to Float (double-precision)") (`Map to Check` :type "Map of Name to Float (double-precision)"))
  (bind _keys (`BlueprintMapLibrary.Map_Keys` Map))
  (for _array_element _keys
    (`self.Add Key if Missing: Float` (`local.Map to Check`) _array_element)))

(fn `Update Map: Float`
  (params (`in Key` :type Name) (`in Change` :type "Float (double-precision)") (`in Map` :type "Map of Name to Float (double-precision)"))
  (returns (`out Map` :type "Map of Name to Float (double-precision)"))
  (locals (`Temp Amount` :type "Float (double-precision)"))
  (bind _in_key (`local.in Key`))
  (set `local.Temp Amount` (`BlueprintMapLibrary.Map_Find` `in Map` `in Key`)) ; Get the value to keep it safe.
  (`BlueprintMapLibrary.Map_Remove` (`local.in Map`) _in_key) ; Remove the Key & Value
  (`BlueprintMapLibrary.Map_Add` (`local.in Map`) _in_key (+ (`local.Temp Amount`) (`local.in Change`))) ; Add the Key with new Value
)

(fn `Update Map: Float with Cap`
  (params (Caller :type "Actor Object Reference") (`in Key` :type Name) (`in Change` :type "Float (double-precision)") (`in Map` :type "Map of Name to Float (double-precision)") (`in Cap` :type "Float (double-precision)"))
  (returns (Excess :type "Float (double-precision)"))
  (locals (`Temp Amount` :type "Float (double-precision)"))
  (set `local.Temp Amount` (`BlueprintMapLibrary.Map_Find` `in Map` `in Key`))
  (`BlueprintMapLibrary.Map_Remove` `in Map` `in Key`)
  (bind (_new_current _actual_amount _over_by) (`/Game/BluePrints/FunctionLibs/FancyMath.Cap and return Excess` (`local.in Change`) (`local.Temp Amount`) (`local.in Cap`) Caller))
  (`BlueprintMapLibrary.Map_Add` `in Map` `in Key` _new_current)
  (return _over_by))