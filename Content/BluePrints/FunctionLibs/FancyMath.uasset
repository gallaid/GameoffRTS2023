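; FancyMath is a math function library for adding to or subtracting from a value within a limit.
; CapAndReturnExcess adds and clamps to a maximum, returning the new value, amount applied and signed difference from the cap.
; FloorAndReturnExcess subtracts and clamps to a minimum, deriving its underage and actual amount from result plus minimum, rather than minus.
; Both pass every output through RoundTo2Places, which rounds to two decimals.
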(fn `Cap and return Excess`
  (params (`In Amount` :type "Float (double-precision)") (`In Current` :type "Float (double-precision)") (`In Max` :type "Float (double-precision)"))
  (returns (`New Current` :type "Float (double-precision)") (`Actual Amount` :type "Float (double-precision)") (`Over By` :type "Float (double-precision)"))
  (locals (`Amt+Curr` :type "Float (double-precision)") (Excess :type "Float (double-precision)") (`Output Amt` :type "Float (double-precision)") (Actual :type "Float (double-precision)"))
  (bind _output_get (set `local.Amt+Curr` (+ `In Amount` `In Current`))) ; Total of curr and incoming
  (set `local.Excess` (- _output_get `In Max`)) ; The amount above cap
  ;[1 1 1] Clamps max output to "In Max", and returns the "real" result.
  (if (> (`local.Amt+Curr`) `In Max`)
    (set `local.Output Amt` (`local.in Max`))
    (set `local.Actual` (- (`local.in Amount`) (`local.Excess`)))
    (else
      (set `local.Output Amt` (`local.Amt+Curr`))
      (set `local.Actual` (`local.in Amount`))))
  (return (`self.Round to 2 Places` (`local.Output Amt`)) (`self.Round to 2 Places` (`local.Actual`)) (`self.Round to 2 Places` (`local.Excess`))))

(fn `Floor and return Excess`
  (params (`In Current` :type "Float (double-precision)") (`In Amount` :type "Float (double-precision)") (`In Min` :type "Float (double-precision)"))
  (returns (`New Current` :type "Float (double-precision)") (`Actual Amt` :type "Float (double-precision)") (`Under By` :type "Float (double-precision)"))
  (locals (`Amt+Curr` :type "Float (double-precision)") (Underage :type "Float (double-precision)") (`Output Amt` :type "Float (double-precision)") (Actual :type "Float (double-precision)"))
  (bind _output_get (set `local.Amt+Curr` (- `In Current` `In Amount`))) ; Total of curr and incoming
  (set `local.Underage` (+ _output_get `In Min`)) ; The amount below minimum
  ;[1 1 1] Clamps max output to In Min while creating some debug data.
  (if (< (`local.Amt+Curr`) `In Min`)
    (set `local.Output Amt` (`local.In Min`))
    (set `local.Actual` (- (`local.In Amount`) (`local.Underage`)))
    (else
      (set `local.Output Amt` (`local.Amt+Curr`))
      (set `local.Actual` (`local.In Amount`))))
  (return (`self.Round to 2 Places` (`local.Output Amt`)) (`self.Round to 2 Places` (`local.Actual`)) (`self.Round to 2 Places` (`local.Underage`))))

(fn `Round to 2 Places`
  (params (`To be Rounded` :type "Float (double-precision)"))
  (returns (Rounded :type "Float (double-precision)"))
  (return (/ (`KismetMathLibrary.Conv_IntToDouble` (`KismetMathLibrary.Round` (* `To be Rounded` 100.0))) 100.0)))