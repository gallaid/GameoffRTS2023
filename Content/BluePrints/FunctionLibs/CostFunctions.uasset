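; Function library for resource costs: checking and spending from resource maps, and reading cost maps from friendly units or buildings.
; Single-resource checks feed the multi-cost check, which counts failures but returns true when any exist, contrary to its comment.
; Buying gates Apply Costs on that result, then passes each cost to UpdateMapFloat.
; Apply Costs itself does no affordability check and relies on callers to guard it.
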(fn `Cost: Apply Costs`
  (params (`Cost Map` :type "Map of Name to Float (double-precision)") (`Resource Map` :type "Map of Name to Float (double-precision)"))
  (returns (`Out Resource Map` :type "Map of Name to Float (double-precision)"))
  (locals (`Interim Resource Map` :type "Map of Name to Float (double-precision)"))
  (bind _keys (`BlueprintMapLibrary.Map_Keys` `Cost Map`))
  ;[0.498 1 0] Loop Body -- Pays the cost in the Cost Map from Resource Map.
  (for _array_element _keys
    (bind _out_map (`/Game/BluePrints/FunctionLibs/MapFunctions.Update Map: Float` _array_element (`BlueprintMapLibrary.Map_Find` `Cost Map` _array_element) (`local.Resource Map`)))
    (set `local.Interim Resource Map` _out_map))
  ;[1 1 1] Note that weird shit will happen if you run this without putting it behind a "Do I Have Enough" call.
  (return (`local.Interim Resource Map`)))

(fn `Cost: Do I Have Enough Of These?`
  (params (`Resource Map` :type "Map of Name to Float (double-precision)") (`Cost Map` :type "Map of Name to Float (double-precision)"))
  (returns (`Do I have enough?` :type Boolean))
  (locals (`Unsuccessful Checks` :type Integer))
  (set `local.Unsuccessful Checks` 0)
  (bind _keys (`BlueprintMapLibrary.Map_Keys` `Cost Map`))
  ;[0.6564 1 0] Loop Body, checks all the things in the CostMap and increments UnsuccessfulChecks on fail.
  (for _array_element _keys
    (bind _has_enough_ (`self.Cost: Do I Have Enough Of This?` `Resource Map` _array_element (`BlueprintMapLibrary.Map_Find` `Cost Map` _array_element)))
    (if (not _has_enough_)
      (`/Engine/EditorBlueprintResources/StandardMacros.IncrementInt` (`local.Unsuccessful Checks`))))
  ;[1 1 1] If the number of unsuccessful checks is 0 or less, you have enough.
  (return (< 0 (`local.Unsuccessful Checks`))))

(fn `Cost: Do I Have Enough Of This?`
  (params (`Resource Map` :type "Map of Name to Float (double-precision)") (Resource :type Name) (Amount :type "Float (double-precision)"))
  (returns (`Has Enough?` :type Boolean))
  (locals (`Enough?` :type Boolean) (`Resource Amount` :type "Float (double-precision)"))
  (if (`.ReturnValue` (`BlueprintMapLibrary.Map_Find` `Resource Map` Resource))
    (bind _output_get (set `local.Resource Amount` (`BlueprintMapLibrary.Map_Find` (`local.Resource Map`) (`local.Resource`))))
    (set `local.Enough?` (>= _output_get (`local.Amount`)))
    (else
      (set `local.Enough?` false)))
  (return (`local.Enough?`)))

(fn `Cost: Try Get Cost Map from Actor`
  (params (Actor :type "Actor Object Reference"))
  (returns (`Cost Map` :type "Map of Name to Float (double-precision)") (`Found Map` :type Boolean))
  (locals (`Cost Map Out` :type "Map of Name to Float (double-precision)") (`Did I find a Cost Map?` :type Boolean))
  ;[1 1 1] Checks Friendly Units and Buildings for their Cost Maps; unexpected behavior may occur if the Cost Map is empty.
  (bind _asbp_friendly_unit_base (cast `/Game/BluePrints/Map_Entities/Friendly/BP_Friendly_Unit_Base` Actor)
    (:`then`
      (set `local.Cost Map Out` (`/Game/BluePrints/Map_Entities/Friendly/BP_Friendly_Unit_Base.Cost Map` _asbp_friendly_unit_base))
      (set `local.Did I find a Cost Map?` true :!label _label))
    (:`CastFailed`
      (bind _asbp_building_base (cast `/Game/BluePrints/Map_Entities/Buildings/BP_BuildingBase` Actor)
        (:`then`
          (set `local.Cost Map Out` (`/Game/BluePrints/FunctionLibs/ActorComponents/Buildable.Cost to Build` (`/Game/BluePrints/Map_Entities/Buildings/BP_BuildingBase.Buildable` _asbp_building_base)))
          (goto _label))
        (:`CastFailed`
          (set `local.Did I find a Cost Map?` false)))))
  (return (`local.Cost Map Out`) (`local.Did I find a Cost Map?`)))

(fn `Cost: Try to Buy with Resources`
  (params (`Resource Map` :type "Map of Name to Float (double-precision)") (`Cost Map` :type "Map of Name to Float (double-precision)"))
  (returns (`Success?` :type Boolean) (`Out Resource Map` :type "Map of Name to Float (double-precision)"))
  (locals (`Buy Success?` :type Boolean))
  (bind _do_i_have_enough_ (`self.Cost: Do I Have Enough Of These?` `Resource Map` `Cost Map`)) ; Checks to see if you can afford it
  ;[1 1 1] Only uses "Apply Costs" if it knows you can afford it to prevent "key not found" errors.
  (if _do_i_have_enough_
    (bind _out_resource_map (`self.Cost: Apply Costs` (`local.Cost Map`) (`local.Resource Map`)))
    (set `local.Buy Success?` true)
    (else
      (set `local.Buy Success?` false)))
  (return (`local.Buy Success?`) _out_resource_map))

(fn `Cost: Try to Spend Resource`
  (params (`Resource Map` :type "Map of Name to Float (double-precision)") (Resource :type Name) (Amount :type "Float (double-precision)"))
  (returns (`Success?` :type Boolean))
  (locals (`Resource spent?` :type Boolean))
  (bind _has_enough_ (`self.Cost: Do I Have Enough Of This?` `Resource Map` Resource Amount))
  (if _has_enough_
    (`/Game/BluePrints/FunctionLibs/MapFunctions.Update Map: Float` (`local.Resource`) (`local.Amount`) (`local.Resource Map`))
    (set `local.Resource spent?` true)
    (else
      (set `local.Resource spent?` false)))
  (return (`local.Resource spent?`)))