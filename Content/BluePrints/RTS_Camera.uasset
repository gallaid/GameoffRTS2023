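; RTS camera actor that becomes the first player's view target on BeginPlay and handles player-driven panning and zooming.
; Forward and left input actions offset the actor along world X and Y by MovementSpeed, without sweep or delta-time scaling.
; The zoom action adjusts the SpringArm's target length by ScrollSpeed, with no clamping.
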(event `self.ReceiveBeginPlay`
  (`PlayerController.SetViewTargetWithBlend` (`GameplayStatics.GetPlayerController` 0) self 0.0 "VTBlend_Linear" 0.0 false))

(event `EnhancedInput|/Game/BluePrints/Input/Actions/Camera_MoveForwardAxis`
  (params (ActionValue :type "Float (double-precision)") (ElapsedSeconds :type "Float (double-precision)") (TriggeredSeconds :type "Float (double-precision)") (InputAction :type "InputAction Object Reference" :default "/Game/BluePrints/Input/Actions/Camera_MoveForwardAxis.Camera_MoveForwardAxis"))
  (:`Triggered`
    (`self.K2_SetActorLocation` (+ (`KismetMathLibrary.MakeVector` (* ActionValue (`self.MovementSpeed`))) (`self.K2_GetActorLocation`)))))

(event `EnhancedInput|/Game/BluePrints/Input/Actions/Camera_MoveLeftAxis`
  (params (ActionValue :type "Float (double-precision)") (ElapsedSeconds :type "Float (double-precision)") (TriggeredSeconds :type "Float (double-precision)") (InputAction :type "InputAction Object Reference" :default "/Game/BluePrints/Input/Actions/Camera_MoveLeftAxis.Camera_MoveLeftAxis"))
  (:`Triggered`
    (`self.K2_SetActorLocation` (+ (`KismetMathLibrary.MakeVector` 0.0 (* ActionValue (`self.MovementSpeed`))) (`self.K2_GetActorLocation`)))))

(event `EnhancedInput|/Game/BluePrints/Input/Actions/Camera_CameraZoom`
  (params (ActionValue :type "Float (double-precision)") (ElapsedSeconds :type "Float (double-precision)") (TriggeredSeconds :type "Float (double-precision)") (InputAction :type "InputAction Object Reference" :default "/Game/BluePrints/Input/Actions/Camera_CameraZoom.Camera_CameraZoom"))
  (bind _springarm (`self.SpringArm`))
  (:`Triggered`
    (set `SpringArmComponent.TargetArmLength` (+ (* ActionValue (`self.ScrollSpeed`)) (`SpringArmComponent.TargetArmLength` _springarm)) _springarm)))

(fn `UserConstructionScript`)