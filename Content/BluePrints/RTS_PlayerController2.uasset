(event `self.ReceiveBeginPlay`
  (bind _returnvalue (subsystem `EnhancedInputLocalPlayerSubsystem`))
  ;[0.05098 0.05098 0.05098] Add Mapping Context
  (`/Engine/EditorBlueprintResources/StandardMacros.IsValid` _returnvalue
    (:`Is Valid`
      (`EnhancedInputSubsystemInterface.AddMappingContext` _returnvalue "/Game/BluePrints/Input/IMC_Default.IMC_Default" 0 (struct))
      ;[1 1 1] Defines main camera
      (set `self.bShowMouseCursor` true)
      (bind _asrts_camera (cast `/Game/BluePrints/RTS_Camera` (`GameplayStatics.GetPlayerPawn` 0)))
      (bind _output_get (set `self.RTSCamera Actor` _asrts_camera))
      (set `self.Main Camera` (`/Game/BluePrints/RTS_Camera.MainCamera` _output_get)))))

(event `EnhancedInput|/Game/BluePrints/Input/Actions/RightClick`
  (params (ActionValue :type Boolean) (ElapsedSeconds :type "Float (double-precision)") (TriggeredSeconds :type "Float (double-precision)") (InputAction :type "InputAction Object Reference" :default "/Game/BluePrints/Input/Actions/RightClick.RightClick"))
  (bind (_worldlocation _worlddirection) (`self.DeprojectMousePositionToWorld`))
  (:`Triggered`
    (if (> (`KismetArrayLibrary.Array_Length` (`self.Selected Actors`)) 0)
      (bind _outhit (`KismetSystemLibrary.LineTraceSingle` :`Start` (`SceneComponent.K2_GetComponentLocation` (`self.Main Camera`)) :`End` (+ _worldlocation (* _worlddirection 5000.0)) :`TraceChannel` "TraceTypeQuery2" :`bTraceComplex` true :`DrawDebugType` "Persistent"))
      (for _array_element (`self.Selected Actors`)
        ;[1 1 1] Version that works on BP_Friendly_Unit_Base
        (bind _asbp_peon (cast `/Game/BluePrints/Map_Entities/Friendly/Peon/BP_Peon` _array_element))
        (`/Game/BluePrints/Map_Entities/Friendly/BP_Friendly_Unit_Base.RightClickedWhileSelected` _asbp_peon _outhit)))))

(event `EnhancedInput|/Game/BluePrints/Input/Actions/ControlLeftClick`
  (params (ActionValue :type Boolean) (ElapsedSeconds :type "Float (double-precision)") (TriggeredSeconds :type "Float (double-precision)") (InputAction :type "InputAction Object Reference" :default "/Game/BluePrints/Input/Actions/ControlLeftClick.ControlLeftClick")))

(event `EnhancedInput|/Game/BluePrints/Input/Actions/LeftClick`
  (params (ActionValue :type Boolean) (ElapsedSeconds :type "Float (double-precision)") (TriggeredSeconds :type "Float (double-precision)") (InputAction :type "InputAction Object Reference" :default "/Game/BluePrints/Input/Actions/LeftClick.LeftClick"))
  (:`Started`
    (if (`self.Build Mode?`)
      (`KismetSystemLibrary.PrintString` "left clicked but in build mode")
      (else
        ;[1 1 1] Create and destroy "Selector Box" to get and select Friendly Units
        (set `self.Start Drag` (`.Location` (`GameplayStatics.BreakHitResult` (`self.GetHitResultUnderCursorByChannel` "TraceTypeQuery1"))))
        (`self.Left Click`)
        (bind _returnvalue (`|SpawnActorFromClass` "/Game/BluePrints/SelectionBox.SelectionBox_C" (`KismetMathLibrary.MakeTransform` (`self.Start Drag`)) "Undefined" "MultiplyWithRoot" null null))
        (set `self.SelectorBox` _returnvalue))))
  (:`Completed`
    (if (`self.Build Mode?`)
      (`KismetSystemLibrary.PrintString` "left click ended but in build mode")
      (set `self.On Cursor Object` null)
      (else
        (`/Engine/EditorBlueprintResources/StandardMacros.IsValid` (`self.SelectorBox`)
          (:`Is Valid`
            (`self.K2_DestroyActor` (`self.SelectorBox`))))))))

(event `EnhancedInput|/Game/BluePrints/Input/Actions/IA_BuildMenu`
  (params (ActionValue :type Boolean) (ElapsedSeconds :type "Float (double-precision)") (TriggeredSeconds :type "Float (double-precision)") (InputAction :type "InputAction Object Reference" :default "/Game/BluePrints/Input/Actions/IA_BuildMenu.IA_BuildMenu"))
  (bind _returnvalue (`self.GetHUD`))
  ;[1 1 1] Build Mode Toggle
  (:`Completed`
    ;;[1 1 1] If you're in build mode, make the menu go away, if not, populate it.
    (if (`self.Build Mode?`)
      (bind _asbp_hud (cast `/Game/BluePrints/BP_HUD` _returnvalue))
      (`PanelWidget.ClearChildren` (`/Game/BluePrints/UI/UI_Interactive_Main.BuildTray` (`/Game/BluePrints/BP_HUD.Interactive UI` _asbp_hud)))
      ;;[1 1 1] Destroys the on cursor object if it's not placed yet.
      (`self.K2_DestroyActor` (`self.On Cursor Object`))
      (else
        (bind _asbp_hud_2 (cast `/Game/BluePrints/BP_HUD` _returnvalue))
        (`/Game/BluePrints/UI/UI_Interactive_Main.Populate Build Tray` (`/Game/BluePrints/BP_HUD.Interactive UI` _asbp_hud_2))))
    (set `self.Build Mode?` (not (`self.Build Mode?`)))))

(event `self.ReceiveTick`
  (params (DeltaSeconds :type "Float (single-precision)"))
  (bind _on_cursor_object (`self.On Cursor Object`))
  (if (and (`self.Build Mode?`) (`KismetSystemLibrary.IsValid` _on_cursor_object))
    (`self.Move Target Placeable To Cursor` _on_cursor_object)))

(fn `Check For Deselect`
  (params (`Actor Array` :type "Array of Actor Object Reference"))
  (bind _selected_actors (`self.Selected Actors`))
  ;[1 1 1 1 16] Loops through Selected Actors, comparing it to the 'Incoming" Array; if "Incoming" has an element which "Selected" has, do nothing, if it does not, remove that Actor from the "Selected" Array.
  (for _array_element _selected_actors
    (`KismetSystemLibrary.PrintString` (`KismetStringLibrary.Concat_StrStr` (`KismetStringLibrary.Conv_IntToString` (`KismetArrayLibrary.Array_Length` `Actor Array`)) "in" (`KismetStringLibrary.Conv_IntToString` (`KismetArrayLibrary.Array_Length` _selected_actors))))
    (if (not (`KismetArrayLibrary.Array_Contains` `Actor Array` _array_element))
      (`self.DeselectActor` _array_element)))
  ;[1 1 1] Updates "Unit Selection Tray" after it's done
  (bind _asbp_hud (cast `/Game/BluePrints/BP_HUD` (`self.GetHUD`)))
  (`/Game/BluePrints/UI/UI_Interactive_Main.Populate Unit Selection Tray` (`/Game/BluePrints/BP_HUD.Interactive UI` _asbp_hud)))

(fn `Control Click`
  (bind _hit (`self.Get Line Trace From Mouse`))
  ;[1 1 1] BP_Friendly_Unit_Base
  (bind _asbp_friendly_unit_base (cast `/Game/BluePrints/Map_Entities/Friendly/BP_Friendly_Unit_Base` (`.HitActor` (`GameplayStatics.BreakHitResult` _hit))))
  (if (`/Game/BluePrints/Map_Entities/BP_SelectableActor.IsSelected` _asbp_friendly_unit_base)
    (`self.DeselectActor` _asbp_friendly_unit_base)
    (else
      (`self.Select Actor` _asbp_friendly_unit_base)))
  ;[1 1 1] Updates Unit Selection Tray after it's done
  (`/Game/BluePrints/UI/UI_Interactive_Main.Populate Unit Selection Tray` (`/Game/BluePrints/BP_HUD.Interactive UI` (`self.As BP HUD`))))

(fn `DeselectActor`
  (params (`Deselect This Actor` :type "Actor Object Reference"))
  (bind _asbp_friendly_unit_base (cast `/Game/BluePrints/Map_Entities/Friendly/BP_Friendly_Unit_Base` `Deselect This Actor`))
  (set `/Game/BluePrints/Map_Entities/BP_SelectableActor.IsSelected` false _asbp_friendly_unit_base)
  (`KismetArrayLibrary.Array_RemoveItem` (`self.Selected Actors`) `Deselect This Actor`))

(fn `Get Mouse Position`
  (returns (`Mouse Position` :type "Vector Structure"))
  (bind (_worldlocation _worlddirection) (`self.DeprojectMousePositionToWorld`))
  (bind _outhit (`KismetSystemLibrary.LineTraceSingle` (`SceneComponent.K2_GetComponentLocation` (`self.Main Camera`)) (+ _worldlocation (* _worlddirection 5000.0)) "TraceTypeQuery2" true))
  (return (`.Location` (`GameplayStatics.BreakHitResult` _outhit))))

(fn `Left Click`
  (for _array_element (`self.Selected Actors`)
    (`self.DeselectActor` _array_element))
  (bind _hit (`self.Get Line Trace From Mouse`))
  ;[1 1 1] Selects what you clicked on
  (bind _asbp_friendly_unit_base (cast `/Game/BluePrints/Map_Entities/Friendly/BP_Friendly_Unit_Base` (`.HitActor` (`GameplayStatics.BreakHitResult` _hit))))
  (`self.Select Actor` _asbp_friendly_unit_base)
  (`KismetSystemLibrary.PrintString` "is this working"))

(fn `Move Target Placeable To Cursor`
  (params (`in Placeable` :type "/Game/BluePrints/Map_Entities/BP_Placeable Object Reference"))
  (bind _mouse_position (`self.Get Mouse Position`))
  (`self.K2_SetActorTransform` `in Placeable` (`KismetMathLibrary.MakeTransform` (`KismetMathLibrary.MakeVector` (.x _mouse_position) (.y _mouse_position) (.z (.location (`self.GetTransform` `in Placeable`))))) false false))

(fn `Select Actor`
  (params (IncomingActor :type "Actor Object Reference"))
  ;[1 1 1] Version that works on BP_Friendly_Base_Unit
  (bind _asbp_friendly_unit_base (cast `/Game/BluePrints/Map_Entities/Friendly/BP_Friendly_Unit_Base` IncomingActor)
    (:`then`
      (set `/Game/BluePrints/Map_Entities/BP_SelectableActor.IsSelected` true _asbp_friendly_unit_base)
      (`KismetArrayLibrary.Array_AddUnique` (`self.Selected Actors`) _asbp_friendly_unit_base))
    (:`CastFailed`
      (`KismetSystemLibrary.PrintString` "cast to BP_F failed on select actor" true true (struct :`G` 1.0 :`B` 0.024355 :`A` 1.0) 12.0))))

(fn `Set Destination`
  (params (Destination :type "Vector Structure"))
  (for _array_element (`self.Selected Actors`)
    (bind _asbp_friendly_unit_base (cast `/Game/BluePrints/Map_Entities/Friendly/BP_Friendly_Unit_Base` _array_element))
    (`/Game/BluePrints/Map_Entities/Friendly/BP_Friendly_Unit_Base.Move To` _asbp_friendly_unit_base (`local.Destination`))))

(fn `Spawn Placeable on Cursor`
  (params (`What it Spawns` :type "/Game/BluePrints/Map_Entities/BP_Placeable Class Reference"))
  (returns (`On Cursor Object` :type "/Game/BluePrints/Map_Entities/BP_Placeable Object Reference"))
  (bind _mouse_position (`self.Get Mouse Position`))
  (bind _returnvalue (`|SpawnActorFromClass` `What it Spawns` (`KismetMathLibrary.Conv_VectorToTransform` _mouse_position) "Undefined" "MultiplyWithRoot" null "" null))
  (return _returnvalue))

(fn `UserConstructionScript`)