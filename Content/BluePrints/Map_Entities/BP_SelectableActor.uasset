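; BP_SelectableActor is an actor Blueprint for a selectable map entity that shows a status bar widget while selected.
; Each Tick calls the parent Tick, then sets WidgetStatusBar visibility from the IsSelected flag by polling, without propagating to child components.
; Nothing here sets IsSelected, and the construction script only calls its parent.
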(event `self.ReceiveTick`
  (params (DeltaSeconds :type "Float (single-precision)"))
  (bind _widget_status_bar (`self.Widget Status Bar`))
  (`parent.ReceiveTick` DeltaSeconds)
  (if (`self.IsSelected`)
    (`SceneComponent.SetVisibility` _widget_status_bar true false)
    (else
      (`SceneComponent.SetVisibility` _widget_status_bar false false))))

(fn `UserConstructionScript`
  (`parent.UserConstructionScript`))