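; BP_CombatActorBase is a base for combat entities with damage resistances and a status bar widget.
; On BeginPlay it fills the Resists map with any damage types missing from the Damage_Types_UI table at zero, so only non-default resists need authoring.
; Tick runs DamageUtilities regen and non-player health bar updates, and holds the bar at a fixed world rotation.
; A deprecated function spawns projectiles; the timed firing logic is disconnected.
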(event `self.ReceiveBeginPlay`
  (bind _resists (`self.Resists`))
  ;[1 1 1 1 16] Checks the pawn's "Resists" map and adds any damage types which are missing. This allows us to add resists to pawns without having to add them all, making it easy to view.
  (bind _outrownames (`DataTableFunctionLibrary.GetDataTableRowNames` "/Game/BluePrints/DataTables/Damage_Types_UI.Damage_Types_UI"))
  (for _array_element _outrownames
    (if (not (`.ReturnValue` (`BlueprintMapLibrary.Map_Find` _resists _array_element)))
      (`BlueprintMapLibrary.Map_Add` _resists _array_element)))
  ;[1 1 1] Sets health bar to face the right way
  (`SceneComponent.K2_SetWorldRotation` (`self.Widget Status Bar`) (struct :`Pitch` 45.0 :`Yaw` -180.0) false false))

(event `self.ReceiveTick`
  (params (DeltaSeconds :type "Float (single-precision)"))
  (`/Game/BluePrints/FunctionLibs/ActorComponents/DamageUtilities.Regen` (`self.DamageUtilities`) self)
  (`/Game/BluePrints/FunctionLibs/ActorComponents/DamageUtilities.update Non-Player-Health-Bars` (`self.DamageUtilities`) self)
  (`SceneComponent.K2_SetWorldRotation` (`self.Widget Status Bar`) (struct :`Pitch` 45.0 :`Yaw` 180.0) false false))

(fn `Fire Projectile (depracated)`
  (params (projectileType :type "Actor Class Reference") (projectileDamage :type "Float (double-precision)") (PlayerProjectile :type Boolean) (SpawnLocation :type "Vector Structure") (SpawnRotator :type "Rotator Structure"))
  (bind _returnvalue (`|SpawnActorFromClass` projectileType (`KismetMathLibrary.MakeTransform` SpawnLocation SpawnRotator) "AlwaysSpawn" "MultiplyWithRoot" self self))
  (bind _asbp_projectile_base (cast `/Game/BluePrints/Projectiles/BP_ProjectileBase` _returnvalue))
  (set `/Game/BluePrints/Projectiles/BP_ProjectileBase.projectileDamage` projectileDamage _asbp_projectile_base)
  (set `/Game/BluePrints/Projectiles/BP_ProjectileBase.PlayerProjectile` PlayerProjectile _asbp_projectile_base)
  (set `/Game/BluePrints/Projectiles/BP_ProjectileBase.Attacker` self _asbp_projectile_base))

(fn `UserConstructionScript`)