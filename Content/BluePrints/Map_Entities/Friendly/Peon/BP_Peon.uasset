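; BP_Peon is a friendly worker unit that gathers resources, returns them to the main building and works on construction.
; Right-clicks while selected write a resource target or move destination to the AI controller's Blackboard.
; Task functions fill inventory through resource-map transfers, clear it only on successful delivery, and find the closest replacement resource via the main building.
; Construction helpers accept delivery tasks and add labor, while TransferResourcesForConstruction is an empty stub.
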(event `self.ReceiveBeginPlay`
  (bind _returnvalue (`AIBlueprintHelperLibrary.GetBlackboard` (`AIBlueprintHelperLibrary.GetAIController` self)))
  (`parent.ReceiveBeginPlay`)
  (`BlackboardComponent.SetValueAsName` _returnvalue "Current Resource Type Assigned" "None")
  (`BlackboardComponent.SetValueAsObject` _returnvalue "MainBuilding" (`self.Main Building`)))

(event `self.ReceiveTick`
  (params (DeltaSeconds :type "Float (single-precision)"))
  (`parent.ReceiveTick` DeltaSeconds))

(fn `Accept Delivery Task`
  (params (Building :type "Actor Object Reference"))
  (bind _asbp_building_base (cast `/Game/BluePrints/Map_Entities/Buildings/BP_BuildingBase` Building))
  (`/Game/BluePrints/FunctionLibs/ActorComponents/Buildable.Peon: Accept Delivery Tasking` (`/Game/BluePrints/Map_Entities/Buildings/BP_BuildingBase.Buildable` _asbp_building_base) self))

(fn `Add Labor to Building`
  (params (`in Actor` :type "Actor Object Reference"))
  (bind _asbp_building_base (cast `/Game/BluePrints/Map_Entities/Buildings/BP_BuildingBase` `in Actor`)
    (:`then`
      (`/Game/BluePrints/FunctionLibs/ActorComponents/Buildable.Standalone: Add Labor` (`/Game/BluePrints/Map_Entities/Buildings/BP_BuildingBase.Buildable` _asbp_building_base) (`self.Labor Rate`)))
    (:`CastFailed`
      (`KismetSystemLibrary.PrintString` "Peon attempted to Add Labor to a map entity that is not a building."))))

(fn `Find New Resource`
  (returns (HasResource :type Boolean))
  (bind _out_resource (`/Game/BluePrints/Map_Entities/BP_MainBuilding.Get Next Closest Resource` (`self.Main Building`) (`self.Current Type Assigned`)))
  (bind _output_get (set `self.Current Resource` _out_resource))
  (`/Engine/EditorBlueprintResources/StandardMacros.IsValid` _output_get
    (:`Is Valid`
      (return true))
    (:`Is Not Valid`
      (return false))))

(fn `Gather Resource`
  (returns (IsFull :type Boolean))
  (locals (`Amount Requested` :type "Float (double-precision)"))
  (bind _resourceholder (`self.ResourceHolder`))
  ;[1 1 1] Build Transfer Map, input Actors, function does the rest.
  (`/Game/BluePrints/FunctionLibs/ResourceFunctions.RA: Take Map from Target` (`self.Current Resource`) self (`|MakeMap` (`/Game/BluePrints/Resources/BP_ResourceBase.TypeName` (`self.Current Resource`)) (`self.Rate for Gather`)))
  (return (>= (`/Game/BluePrints/FunctionLibs/ActorComponents/ResourceHolder.curr Inventory` _resourceholder) (`/Game/BluePrints/FunctionLibs/ActorComponents/ResourceHolder.Inventory Limit` _resourceholder))))

(fn `RightClickedWhileSelected`
  (params (`Hit IN` :type "HitResult Structure"))
  (bind (_bblockinghit _binitialoverlap _time _distance _location _impactpoint _normal _impactnormal _physmat _hitactor) (`GameplayStatics.BreakHitResult` `Hit IN`))
  (bind _blackboard (`AIController.Blackboard` (`AIBlueprintHelperLibrary.GetAIController` self)))
  (bind _asbp_resource_base (cast `/Game/BluePrints/Resources/BP_ResourceBase` _hitactor)
    (:`then`
      (bind _output_get (set `self.Current Resource` _asbp_resource_base))
      (`BlackboardComponent.SetValueAsObject` (`AIController.Blackboard` (`AIBlueprintHelperLibrary.GetAIController` self)) "ResourceCollectionTarget" _output_get)
      (bind _output_get_2 (set `self.Current Type Assigned` (`/Game/BluePrints/Resources/BP_ResourceBase.TypeName` _asbp_resource_base)))
      (`BlackboardComponent.SetValueAsName` (`AIController.Blackboard` (`AIBlueprintHelperLibrary.GetAIController` self)) "Current Resource Type Assigned" _output_get_2))
    (:`CastFailed`
      (`BlackboardComponent.SetValueAsVector` _blackboard "Destination" _location)
      (`BlackboardComponent.SetValueAsName` _blackboard "Current Resource Type Assigned" "None"))))

(fn `Transfer Inventory to Main Building`
  ;[1 1 1] Try to transfer inventory to main building.
  (bind (_success_ _debug) (`/Game/BluePrints/FunctionLibs/ResourceFunctions.RA: Try Transfer Resource(S)` self (`self.Main Building`) (`/Game/BluePrints/FunctionLibs/ActorComponents/ResourceHolder.Resource Map` (`self.ResourceHolder`))))
  ;[1 1 1] But only actually clear inventory if the transfer succeeds.
  (if _success_
    (`BlueprintMapLibrary.Map_Clear` (`/Game/BluePrints/FunctionLibs/ActorComponents/ResourceHolder.Resource Map` (`self.ResourceHolder`)))
    (else
      ;[1 0 0.6526] Debug
      (`KismetSystemLibrary.PrintString` (`KismetStringLibrary.Concat_StrStr` "Failed to return resources to main building. " _debug)))))

(fn `Transfer Resources For Construction`)

(fn `UserConstructionScript`
  (`parent.UserConstructionScript`))