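; BP_UnitBase is a base Blueprint for map unit entities that sets up each unit's status bar widget.
; On BeginPlay it runs the parent logic, casts the WidgetStatusBar component's widget to UI_HealthBar and assigns the unit's Icon as its TypeIcon.
; Overlap and Tick events are disabled, and the construction script only calls the parent.
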(event `self.ReceiveBeginPlay`
  (`parent.ReceiveBeginPlay`)
  (bind _asui_health_bar (cast `/Game/BluePrints/UI/UI_HealthBar` (`WidgetComponent.GetWidget` (`self.Widget Status Bar`))))
  (set `/Game/BluePrints/UI/UI_HealthBar.Type Icon` (`self.Icon`) _asui_health_bar))

(fn `UserConstructionScript`
  (`parent.UserConstructionScript`))